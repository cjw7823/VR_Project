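; Master drum kit actor that spawns kick pedal and hi-hat, turning drumstick hits into sound, haptics and per-drum calls.
; Hits re-arm on end overlap, and stick velocity picks light or hard feedback from DT_HitDrumPart, while pedal overlap plays the kick at fixed strength.
; Left tom, right tom and one cymbal double as previous, next and select inputs for BP_MainWidget.
; Colored AngelRing meshes form a toggleable beginner guide.
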(event OnComponentBeginOverlap(22inch_Kick_Drum_Shell)
  (params (OverlappedComponent :type Primitive%20Component%20Object%20Reference) (OtherActor :type Actor%20Object%20Reference) (OtherComp :type Primitive%20Component%20Object%20Reference) (OtherBodyIndex :type Integer) (bFromSweep :type Boolean) (SweepResult :type Hit%20Result%20Structure%20%28by%20ref%29))
  (Utilities|Casting|CastToBP_KickDrumPedal OtherActor)
  (CallFunction|KickDrumShellSound OverlappedComponent)
  (Class|PlayerController|PlayHapticEffect (Game|GetPlayerController 0) "/Game/Drum_the_Beat/Haptics/Cymbal_Haptic_Hardly.Cymbal_Haptic_Hardly" "Right" 1.0 false)
  (Default|CallBase))

(event OnComponentHit(Snare_Drum_Shell)
  (params (HitComponent :type Primitive%20Component%20Object%20Reference) (OtherActor :type Actor%20Object%20Reference) (OtherComp :type Primitive%20Component%20Object%20Reference) (NormalImpulse :type Vector :default "0, 0, 0") (Hit :type Hit%20Result%20Structure%20%28by%20ref%29))
  (if (Variables|Default|GetOverlapCheck_0)
    (bind _asbp_drum_stick (Utilities|Casting|CastToBP_DrumStick OtherActor))
    (bind _haptic (CallFunction|SoundbyVelocity HitComponent (Variables|/Game/Drum_the_Beat/BluePrint/Drum/BP_DrumStick.BP_DrumStick_C|GetStaticMesh _asbp_drum_stick)))
    (Class|BPIHaptic|Haptic(Message) _asbp_drum_stick _haptic)
    (Variables|Default|SetOverlapCheck_0 false)
    (Default|CallSnare)))

(event OnComponentHit(Floor_Tom)
  (params (HitComponent :type Primitive%20Component%20Object%20Reference) (OtherActor :type Actor%20Object%20Reference) (OtherComp :type Primitive%20Component%20Object%20Reference) (NormalImpulse :type Vector :default "0, 0, 0") (Hit :type Hit%20Result%20Structure%20%28by%20ref%29))
  (if (Variables|Default|GetOverlapCheck_3)
    (bind _asbp_drum_stick (Utilities|Casting|CastToBP_DrumStick OtherActor))
    (bind _haptic (CallFunction|SoundbyVelocity HitComponent (Variables|/Game/Drum_the_Beat/BluePrint/Drum/BP_DrumStick.BP_DrumStick_C|GetStaticMesh _asbp_drum_stick)))
    (Class|BPIHaptic|Haptic(Message) _asbp_drum_stick _haptic)
    (Variables|Default|SetOverlapCheck_3 false)
    (Default|CallFloorTom)))

(event OnComponentEndOverlap(Floor_Tom)
  (params (OverlappedComponent :type Primitive%20Component%20Object%20Reference) (OtherActor :type Actor%20Object%20Reference) (OtherComp :type Primitive%20Component%20Object%20Reference) (OtherBodyIndex :type Integer))
  (Variables|Default|SetOverlapCheck_3 true))

(event OnComponentHit(Cymbal1)
  (params (HitComponent :type Primitive%20Component%20Object%20Reference) (OtherActor :type Actor%20Object%20Reference) (OtherComp :type Primitive%20Component%20Object%20Reference) (NormalImpulse :type Vector :default "0, 0, 0") (Hit :type Hit%20Result%20Structure%20%28by%20ref%29))
  (if (Variables|Default|GetOverlapCheck_4)
    (bind _asbp_drum_stick (Utilities|Casting|CastToBP_DrumStick OtherActor))
    (bind _haptic (CallFunction|SoundbyVelocity HitComponent (Variables|/Game/Drum_the_Beat/BluePrint/Drum/BP_DrumStick.BP_DrumStick_C|GetStaticMesh _asbp_drum_stick)))
    (Class|BPIHaptic|Haptic(Message) _asbp_drum_stick _haptic)
    (Variables|Default|SetOverlapCheck_4 false)
    (Default|CallCrush)))

(event OnComponentEndOverlap(Cymbal1)
  (params (OverlappedComponent :type Primitive%20Component%20Object%20Reference) (OtherActor :type Actor%20Object%20Reference) (OtherComp :type Primitive%20Component%20Object%20Reference) (OtherBodyIndex :type Integer))
  (Variables|Default|SetOverlapCheck_4 true))

(event OnComponentHit(Cymbal3)
  (params (HitComponent :type Primitive%20Component%20Object%20Reference) (OtherActor :type Actor%20Object%20Reference) (OtherComp :type Primitive%20Component%20Object%20Reference) (NormalImpulse :type Vector :default "0, 0, 0") (Hit :type Hit%20Result%20Structure%20%28by%20ref%29))
  (if (Variables|Default|GetOverlapCheck_5)
    (bind _asbp_drum_stick (Utilities|Casting|CastToBP_DrumStick OtherActor))
    (bind _haptic (CallFunction|SoundbyVelocity HitComponent (Variables|/Game/Drum_the_Beat/BluePrint/Drum/BP_DrumStick.BP_DrumStick_C|GetStaticMesh _asbp_drum_stick)))
    (Class|BPIHaptic|Haptic(Message) _asbp_drum_stick _haptic)
    (Variables|Default|SetOverlapCheck_5 false)
    (Default|CallRide)
    (if (!= _haptic 0)
      (Class|BPISelectMusic|Select(Message) (Variables|Default|GetBP_MainWidget)))))

(event OnComponentEndOverlap(Cymbal3)
  (params (OverlappedComponent :type Primitive%20Component%20Object%20Reference) (OtherActor :type Actor%20Object%20Reference) (OtherComp :type Primitive%20Component%20Object%20Reference) (OtherBodyIndex :type Integer))
  (Variables|Default|SetOverlapCheck_5 true))

(event OnComponentEndOverlap(Snare_Drum_Shell)
  (params (OverlappedComponent :type Primitive%20Component%20Object%20Reference) (OtherActor :type Actor%20Object%20Reference) (OtherComp :type Primitive%20Component%20Object%20Reference) (OtherBodyIndex :type Integer))
  (Variables|Default|SetOverlapCheck_0 true))

(event OnComponentHit(Drum_Shell)
  (params (HitComponent :type Primitive%20Component%20Object%20Reference) (OtherActor :type Actor%20Object%20Reference) (OtherComp :type Primitive%20Component%20Object%20Reference) (NormalImpulse :type Vector :default "0, 0, 0") (Hit :type Hit%20Result%20Structure%20%28by%20ref%29))
  (if (Variables|Default|GetOverlapCheck_1)
    (bind _asbp_drum_stick (Utilities|Casting|CastToBP_DrumStick OtherActor))
    (bind _haptic (CallFunction|SoundbyVelocity HitComponent (Variables|/Game/Drum_the_Beat/BluePrint/Drum/BP_DrumStick.BP_DrumStick_C|GetStaticMesh _asbp_drum_stick)))
    (Class|BPIHaptic|Haptic(Message) _asbp_drum_stick _haptic)
    (Variables|Default|SetOverlapCheck_1 false)
    (Default|CallLeftTom)
    (if (!= _haptic 0)
      (Class|BPISelectMusic|Previous(Message) (Variables|Default|GetBP_MainWidget)))))

(event OnComponentEndOverlap(Drum_Shell)
  (params (OverlappedComponent :type Primitive%20Component%20Object%20Reference) (OtherActor :type Actor%20Object%20Reference) (OtherComp :type Primitive%20Component%20Object%20Reference) (OtherBodyIndex :type Integer))
  (Variables|Default|SetOverlapCheck_1 true))

(event OnComponentHit(Drum_Shell1)
  (params (HitComponent :type Primitive%20Component%20Object%20Reference) (OtherActor :type Actor%20Object%20Reference) (OtherComp :type Primitive%20Component%20Object%20Reference) (NormalImpulse :type Vector :default "0, 0, 0") (Hit :type Hit%20Result%20Structure%20%28by%20ref%29))
  (if (Variables|Default|GetOverlapCheck_2)
    (bind _asbp_drum_stick (Utilities|Casting|CastToBP_DrumStick OtherActor))
    (bind _haptic (CallFunction|SoundbyVelocity HitComponent (Variables|/Game/Drum_the_Beat/BluePrint/Drum/BP_DrumStick.BP_DrumStick_C|GetStaticMesh _asbp_drum_stick)))
    (Class|BPIHaptic|Haptic(Message) _asbp_drum_stick _haptic)
    (Variables|Default|SetOverlapCheck_2 false)
    (Default|CallRightTom)
    (if (!= _haptic 0)
      (Class|BPISelectMusic|Next(Message) (Variables|Default|GetBP_MainWidget)))))

(event OnComponentEndOverlap(Drum_Shell1)
  (params (OverlappedComponent :type Primitive%20Component%20Object%20Reference) (OtherActor :type Actor%20Object%20Reference) (OtherComp :type Primitive%20Component%20Object%20Reference) (OtherBodyIndex :type Integer))
  (Variables|Default|SetOverlapCheck_2 true))

(event EventBeginPlay
  (bind _hi_hat_spawnspot (Variables|Default|GetHi-Hat_SpawnSpot))
  (Game|SpawnActorfromClass "/Game/Drum_the_Beat/BluePrint/Drum/BP_KickDrumPedal.BP_KickDrumPedal_C" (Math|Transform|MakeTransform (Transformation|GetWorldLocation (Variables|Default|GetPedal_SpawnSpot)) "0, 0, 0" "1,1,1") "Undefined" 0 0)
  (Game|SpawnActorfromClass "/Game/Drum_the_Beat/BluePrint/Drum/BP_Hi-Hat.BP_Hi-Hat_C" (Math|Transform|MakeTransform (Transformation|GetWorldLocation _hi_hat_spawnspot) (Transformation|GetWorldRotation _hi_hat_spawnspot) "1,1,1") "Undefined" 0 0)
  (CallFunction|SetColorOfAngelRing)
  (bind _returnvalue (Actor|GetActorOfClass "/Game/Drum_the_Beat/BluePrint/BP_MainWidget.BP_MainWidget_C"))
  (Variables|Default|SetBP_MainWidget _returnvalue))

(event EventBeginerGuide
  (if (Variables|Default|GetGuideOn)
    (CallFunction|AngelRingVisible false)
    (Variables|Default|SetGuideOn false)
    (else
      (CallFunction|AngelRingVisible true)
      (Variables|Default|SetGuideOn true))))

(fn ConstructionScript)

(fn SoundbyVelocity
  (params (Hit%20Instrument :type Primitive%20Component%20Object%20Reference) (DrumStick :type Static%20Mesh%20Component%20Object%20Reference))
  (bind _returnvalue (Transformation|GetWorldLocation Hit%20Instrument))
  (bind _returnvalue_2 (Physics|GetPhysicsLinearVelocity DrumStick "None"))
  (if (Math|Vector|VectorIsNearlyZero _returnvalue_2 (Variables|Default|GetIntensity_01))
    (return 0)
    (else
      (bind _returnvalue_3 (Utilities|GetDataTableRow "/Game/Drum_the_Beat/Data/DT_HitDrumPart.DT_HitDrumPart" (Utilities|String|StringToName (Utilities|GetObjectName Hit%20Instrument)))
        (:then
          (if (Math|Vector|VectorIsNearlyZero _returnvalue_2 (Variables|Default|GetIntensity_02))
            (Audio|SpawnSoundatLocation (.SoundLightly (Utilities|Struct|BreakST_HitDrumPart _returnvalue_3)) _returnvalue "0, 0, 0" 1.0 1.0 0.0 0 0)
            (return (.HapticLightly (Utilities|Struct|BreakST_HitDrumPart _returnvalue_3)))
            (else
              (Audio|SpawnSoundatLocation (.SoundHardly (Utilities|Struct|BreakST_HitDrumPart _returnvalue_3)) _returnvalue "0, 0, 0" 1.0 1.0 0.0 0 0)
              (return (.HapticHardly (Utilities|Struct|BreakST_HitDrumPart _returnvalue_3))))))
        (:RowNotFound
          (Development|PrintString "Not Found DataTable" true true "(R=1.000000,G=0.000000,B=0.122107,A=1.000000)" 3e+01))))))

(fn KickDrumShellSound
  (params (Hit%20Instrument :type Primitive%20Component%20Object%20Reference))
  (bind _returnvalue (Utilities|GetDataTableRow "/Game/Drum_the_Beat/Data/DT_HitDrumPart.DT_HitDrumPart" (Utilities|String|StringToName (Utilities|GetObjectName Hit%20Instrument)))
    (:then
      (Audio|SpawnSoundatLocation (.SoundHardly (Utilities|Struct|BreakST_HitDrumPart _returnvalue)) (Transformation|GetWorldLocation Hit%20Instrument) "0, 0, 0" 1.0 1.0 0.01 0 0))))

(fn SetColorOfAngelRing
  (Rendering|Material|SetVectorParameterValueonMaterials (Variables|Default|GetAngelRing) "Rainbow" "1.000000,1.000000, 0")
  (Rendering|Material|SetVectorParameterValueonMaterials (Variables|Default|GetAngelRing1) "Rainbow" "0.000000,1.000000,0.000000")
  (Rendering|Material|SetVectorParameterValueonMaterials (Variables|Default|GetAngelRing2) "Rainbow" "0.000000,0.000000,1.000000")
  (Rendering|Material|SetVectorParameterValueonMaterials (Variables|Default|GetAngelRing3) "Rainbow" "0.100000,0.000000,1.000000")
  (Rendering|Material|SetVectorParameterValueonMaterials (Variables|Default|GetAngelRing4) "Rainbow" "1.000000,0.150000, 0")
  (Rendering|Material|SetVectorParameterValueonMaterials (Variables|Default|GetAngelRing5) "Rainbow" "1.000000,0.000000,0.500000"))

(fn AngelRingVisible
  (params (Visible :type Boolean))
  (Rendering|SetVisibility (Variables|Default|GetAngelRing) Visible false))