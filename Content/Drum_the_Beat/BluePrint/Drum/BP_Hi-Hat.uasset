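; VR drum-kit hi-hat that plays sounds and haptics when struck by a BP_DrumStick, with an overlap flag preventing repeat hits.
; Stick velocity and pedal state pick open/closed, light/hard sounds from DT_Hit_HiHat, returning haptics to the stick.
; Left-shoe press and release move the pedal and bottom cymbal to toggle open state.
; It binds to BP_SeatArea sit/stand events, retrying by timer, and toggles an AngelRing beginner guide.
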(event OnComponentHit(Hi_Hat_Top)
  (params (HitComponent :type Primitive%20Component%20Object%20Reference) (OtherActor :type Actor%20Object%20Reference) (OtherComp :type Primitive%20Component%20Object%20Reference) (NormalImpulse :type Vector :default "0, 0, 0") (Hit :type Hit%20Result%20Structure%20%28by%20ref%29))
  (if (Variables|Default|GetOverlapCheck_6)
    (bind _asbp_drum_stick (Utilities|Casting|CastToBP_DrumStick OtherActor))
    (bind _haptic (CallFunction|SoundbyVelocity HitComponent (Variables|/Game/Drum_the_Beat/BluePrint/Drum/BP_DrumStick.BP_DrumStick_C|GetStaticMesh _asbp_drum_stick)))
    (Class|BPIHaptic|Haptic(Message) _asbp_drum_stick _haptic)
    (Variables|Default|SetOverlapCheck_6 false)))

(event OnComponentEndOverlap(Hi_Hat_Top)
  (params (OverlappedComponent :type Primitive%20Component%20Object%20Reference) (OtherActor :type Actor%20Object%20Reference) (OtherComp :type Primitive%20Component%20Object%20Reference) (OtherBodyIndex :type Integer))
  (Variables|Default|SetOverlapCheck_6 true))

(event EventBeginerGuide
  (if (Variables|Default|GetGuideOn)
    (CallFunction|AngelRingVisible false)
    (Variables|Default|SetGuideOn false)
    (else
      (CallFunction|AngelRingVisible true)
      (Variables|Default|SetGuideOn true))))

(event EventBeginPlay
  (Rendering|SetVisibility (Variables|Default|GetLeft%20Shoes) true false)
  (CallFunction|BindSeatArea)
  (Rendering|Material|SetVectorParameterValueonMaterials (Variables|Default|GetAngelRing) "Rainbow" "1.000000, 0, 0"))

(event EventLeftShoesPressed
  (bind _left_shoes (Variables|Default|GetLeft%20Shoes))
  (Transformation|AddRelativeLocation (Variables|Default|GetHi%20Hat%20Bottom) "0, 0,2.000000" false false)
  (Variables|Default|SetIs%20Open false)
  (Transformation|AddRelativeRotation _left_shoes "0.000000, 0,30.000000" false false)
  (Transformation|AddRelativeLocation _left_shoes "0, 0,-8.000000" false false)
  (Audio|SpawnSoundatLocation "/Game/Drum_the_Beat/DrumSound_wav/HiHatpush_Cue.HiHatpush_Cue" (Transformation|GetWorldLocation (Variables|Default|GetHi_Hat_Top)) "0, 0, 0" 1.0 1.0 0.0 0 0)
  (Class|PlayerController|PlayHapticEffect (Game|GetPlayerController 0) "/Game/Drum_the_Beat/Haptics/Cymbal_Haptic_Lightly.Cymbal_Haptic_Lightly" "Left" 1.0 false))

(event EventLeftShoesReleased
  (bind _left_shoes (Variables|Default|GetLeft%20Shoes))
  (Transformation|AddRelativeLocation (Variables|Default|GetHi%20Hat%20Bottom) "0, 0,-2.000000" false false)
  (Variables|Default|SetIs%20Open true)
  (Transformation|AddRelativeRotation _left_shoes "0.000000, 0,-30.000000" false false)
  (Transformation|AddRelativeLocation _left_shoes "0, 0,8.000000" false false))

(fn ConstructionScript)

(fn SoundbyVelocity
  (params (Hit%20Instrument :type Primitive%20Component%20Object%20Reference) (DrumStick :type Static%20Mesh%20Component%20Object%20Reference))
  (bind _returnvalue (Transformation|GetWorldLocation Hit%20Instrument))
  (bind _returnvalue_2 (Physics|GetPhysicsLinearVelocity DrumStick "None"))
  (if (Math|Vector|VectorIsNearlyZero _returnvalue_2 (Variables|Default|GetIntensity_01))
    (return 0)
    (else
      (bind _returnvalue_3 (Utilities|GetDataTableRow "/Game/Drum_the_Beat/Data/DT_Hit_HiHat.DT_Hit_HiHat" (Utilities|String|StringToName (Utilities|GetObjectName Hit%20Instrument)))
        (:then
          (if (Math|Vector|VectorIsNearlyZero _returnvalue_2 (Variables|Default|GetIntensity_02))
            (if (Variables|Default|GetIs%20Open)
              (Audio|SpawnSoundatLocation (.OpenSoundLightly (Utilities|Struct|BreakST_Hit_HiHat _returnvalue_3)) _returnvalue "0, 0, 0" 1.0 1.0 0.0 0 0)
              (Default|CallOpenHiHat)
              (return (.HapticLightly (Utilities|Struct|BreakST_Hit_HiHat _returnvalue_3)))
              (else
                (Audio|SpawnSoundatLocation (.CloseSoundLightly (Utilities|Struct|BreakST_Hit_HiHat _returnvalue_3)) _returnvalue "0, 0, 0" 1.0 1.0 0.0 0 0)
                (Default|CallCloseHiHat)
                (return (.HapticLightly (Utilities|Struct|BreakST_Hit_HiHat _returnvalue_3)))))
            (elif (Variables|Default|GetIs%20Open)
              (Audio|SpawnSoundatLocation (.OpenSoundHardly (Utilities|Struct|BreakST_Hit_HiHat _returnvalue_3)) _returnvalue "0, 0, 0" 1.0 1.0 0.0 0 0)
              (Default|CallOpenHiHat)
              (return (.HapticHardly (Utilities|Struct|BreakST_Hit_HiHat _returnvalue_3)))
              (else
                (Audio|SpawnSoundatLocation (.CloseSoundHardly (Utilities|Struct|BreakST_Hit_HiHat _returnvalue_3)) _returnvalue "0, 0, 0" 1.0 1.0 0.0 0 0)
                (Default|CallCloseHiHat)
                (return (.HapticHardly (Utilities|Struct|BreakST_Hit_HiHat _returnvalue_3)))))))
        (:RowNotFound
          (Development|PrintString "Not Found DataTable" true true "(R=1.000000,G=0.000000,B=0.122107,A=1.000000)" 3e+01))))))

(fn BindSeatArea
  (bind _returnvalue (Actor|GetActorOfClass "/Game/Drum_the_Beat/BluePrint/BP_SeatArea.BP_SeatArea_C"))
  (Utilities|IsValid _returnvalue
    (:Is%20Valid
      (EventDispatchers|BindEventtoSeatPlayer _returnvalue (EventDispatchers|CreateEvent :!event BPHi-HatAutoGenFunc))
      (EventDispatchers|BindEventtoStandPlayer _returnvalue (EventDispatchers|CreateEvent :!event BPHi-HatAutoGenFunc1)))
    (:Is%20Not%20Valid
      (Utilities|Time|SetTimerbyFunctionName 0 "BindSeatArea" 0.1))))

(fn BPHi-HatAutoGenFunc
  (Rendering|SetVisibility (Variables|Default|GetLeft%20Shoes) true false))

(fn BPHi-HatAutoGenFunc1
  (Rendering|SetVisibility (Variables|Default|GetLeft%20Shoes) false false))

(fn AngelRingVisible
  (params (Visible :type Boolean))
  (Rendering|SetVisibility (Variables|Default|GetAngelRing) Visible false))