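; BP_MainWidget is the in-world song selection menu actor for the drum game, hosting a SelectMusicWidget.
; Input events step through DT_MusicList rows and toggle playback speed between 1.0 and 0.8, stored in BP_GameInstance.
; Select only handles the JingleBell entry: it locks input, spawns score and point actors and plays the track at that pitch.
; It then hides itself and shatters a spawned destructible copy, destroyed after a short delay.
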(event EventNext
  ;[1 1 1] BPI_SelectMusic Next
  (if (Variables|Default|GetCan_Input)
    (bind _asselect_music_widget (Utilities|Casting|CastToSelectMusicWidget (UserInterface|GetUserWidgetObject (Variables|Default|GetSelectMusicWidget))))
    (Default|NextMusic _asselect_music_widget (Variables|Default|GetSelectMusic))
    (if (< (+ (Variables|Default|GetSelectMusic) 1) (Variables|Default|GetDataTableLengh))
      (Variables|Default|SetSelectMusic (+ (Variables|Default|GetSelectMusic) 1))
      (else
        (Variables|Default|SetSelectMusic (Variables|Default|GetSelectMusic))))))

(event EventPrevious
  ;[1 1 1] BPI_SelectMusic_Previous
  (if (Variables|Default|GetCan_Input)
    (bind _asselect_music_widget (Utilities|Casting|CastToSelectMusicWidget (UserInterface|GetUserWidgetObject (Variables|Default|GetSelectMusicWidget))))
    (Default|PreviousMusic _asselect_music_widget (Variables|Default|GetSelectMusic))
    (if (>= (- (Variables|Default|GetSelectMusic) 1) 0)
      (Variables|Default|SetSelectMusic (- (Variables|Default|GetSelectMusic) 1))
      (else
        (Variables|Default|SetSelectMusic (Variables|Default|GetSelectMusic))))))

(event EventBeginPlay
  (bind _outrownames (DataTable|GetDataTableRowNames "/Game/Drum_the_Beat/Data/DT_MusicList.DT_MusicList"))
  (Variables|Default|SetDataTableLengh (Utilities|Array|Length _outrownames)))

(event EventSelect
  (if (Variables|Default|GetCan_Input)
    (switch int (Variables|Default|GetSelectMusic)
      (:2
        (Variables|Default|SetCan_Input false)
        (bind _returnvalue (Actor|GetActorOfClass "/Game/Drum_the_Beat/BluePrint/BP_ScoreSpawnSpot.BP_ScoreSpawnSpot_C"))
        (Game|SpawnActorfromClass "/Game/Drum_the_Beat/BluePrint/BP_JingleBellScore.BP_JingleBellScore_C" (Transformation|GetActorTransform _returnvalue) "Undefined" 0 0)
        (Rendering|SetActorHiddenInGame _returnvalue false)
        (Audio|PlaySound2D "/Game/Drum_the_Beat/Music/JingleBell_MR.JingleBell_MR" 3.0 (Variables|Default|GetMusicSpeed) 4.0 0 0)
        (bind _returnvalue_2 (Actor|GetActorOfClass "/Game/Drum_the_Beat/BluePrint/BP_PointSpawnSpot.BP_PointSpawnSpot_C"))
        (Game|SpawnActorfromClass "/Game/Drum_the_Beat/BluePrint/BP_PointWidget.BP_PointWidget_C" (Transformation|GetActorTransform _returnvalue_2) "Undefined" 0 0)
        (|Spawn_DM)))))

(event EventDecMusicSpeed
  (if (Variables|Default|GetCan_Input)
    (bind _output_get (Variables|Default|SetMusicSpeed 0.8))
    (bind _asselect_music_widget (Utilities|Casting|CastToSelectMusicWidget (UserInterface|GetUserWidgetObject (Variables|Default|GetSelectMusicWidget))))
    (Default|SetMusicSpeed _asselect_music_widget (Utilities|String|ToString(Float) _output_get))
    (bind _asbp_game_instance (Utilities|Casting|CastToBP_GameInstance (Game|GetGameInstance)))
    (Variables|/Game/Drum_the_Beat/BluePrint/BP_GameInstance.BP_GameInstance_C|SetMusicSpeed _asbp_game_instance _output_get)))

(event EventIncMusicSpeed
  (if (Variables|Default|GetCan_Input)
    (bind _output_get (Variables|Default|SetMusicSpeed 1.0))
    (bind _asselect_music_widget (Utilities|Casting|CastToSelectMusicWidget (UserInterface|GetUserWidgetObject (Variables|Default|GetSelectMusicWidget))))
    (Default|SetMusicSpeed _asselect_music_widget (Utilities|String|ToString(Float) _output_get))
    (bind _asbp_game_instance (Utilities|Casting|CastToBP_GameInstance (Game|GetGameInstance)))
    (Variables|/Game/Drum_the_Beat/BluePrint/BP_GameInstance.BP_GameInstance_C|SetMusicSpeed _asbp_game_instance _output_get)))

(fn ConstructionScript)