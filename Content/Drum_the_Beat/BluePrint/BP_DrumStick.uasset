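; BP_DrumStick is the drumstick Blueprint for a motion-controller drum game, handling controller vibration and a hit on the title actor.
; Its Haptic event plays the passed effect on the hand resolved from the owning controller's motion source.
; When no valid BP_Title_DM reference is cached, the same event finds and stores that actor, then applies heavy damage to it.
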(event EventHaptic
  (params (Haptic :type Haptic%20Feedback%20Effect%20Curve%20Object%20Reference))
  (Class|PlayerController|PlayHapticEffect (Game|GetPlayerController 0) Haptic (Utilities|GetHandfromMotionSource (Variables|Default|GetOwnerController)) 1.6 false)
  (Utilities|IsValid (Variables|Default|GetBP_Title_DM)
    (:Is%20Not%20Valid
      (bind _returnvalue (Actor|GetActorOfClass "/Game/Drum_the_Beat/BluePrint/BP_Title_DM.BP_Title_DM_C"))
      (bind _output_get (Variables|Default|SetBP_Title_DM _returnvalue))
      (Game|Damage|ApplyDamage _output_get 1e+03 0 0))))

(fn ConstructionScript)