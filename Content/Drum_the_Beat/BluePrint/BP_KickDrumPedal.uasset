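; BP_KickDrumPedal is the kick drum pedal for the drumming game, animating the pedal and a right shoe.
; Press and release events tilt Pedal2 and move the shoe down, then restore them, using fixed transforms without interpolation.
; BindSeatArea hooks the BP_SeatArea seat and stand events, apparently to toggle shoe visibility, retrying on a short timer until that actor exists.
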(event EventRightShoesPressed
  (bind _right_shoes (Variables|Default|GetRight%20Shoes))
  (Transformation|SetRelativeLocationAndRotation (Variables|Default|GetPedal_2) (Math|Vector|MakeVector -15.0 0.0 4.5) (Math|Rotator|MakeRotator 0.0 -44.0 0.0) false false)
  (Transformation|AddRelativeRotation _right_shoes "0.000000, 0,30.000000" false false)
  (Transformation|AddRelativeLocation _right_shoes "0, 0,-8.000000" false false))

(event EventRightShoesReleased
  (bind _right_shoes (Variables|Default|GetRight%20Shoes))
  (Transformation|SetRelativeLocationAndRotation (Variables|Default|GetPedal_2) (Math|Vector|MakeVector 0.0 0.0 0.0) (Math|Rotator|MakeRotator 0.0 0.0 0.0) false false)
  (Transformation|AddRelativeRotation _right_shoes "0.000000, 0,-30.000000" false false)
  (Transformation|AddRelativeLocation _right_shoes "0, 0,8.000000" false false))

(event EventBeginPlay
  (Rendering|SetVisibility (Variables|Default|GetRight%20Shoes) true false)
  (CallFunction|BindSeatArea))

(fn ConstructionScript)

(fn BindSeatArea
  (bind _returnvalue (Actor|GetActorOfClass "/Game/Drum_the_Beat/BluePrint/BP_SeatArea.BP_SeatArea_C"))
  (Utilities|IsValid _returnvalue
    (:Is%20Valid
      (EventDispatchers|BindEventtoSeatPlayer _returnvalue (EventDispatchers|CreateEvent :!event BPKickDrumPedalAutoGenFunc))
      (EventDispatchers|BindEventtoStandPlayer _returnvalue (EventDispatchers|CreateEvent :!event BPKickDrumPedalAutoGenFunc1)))
    (:Is%20Not%20Valid
      (Utilities|Time|SetTimerbyFunctionName 0 "BindSeatArea" 0.1))))

(fn BPKickDrumPedalAutoGenFunc
  (Rendering|SetVisibility (Variables|Default|GetRight%20Shoes) true false))

(fn BPKickDrumPedalAutoGenFunc1
  (Rendering|SetVisibility (Variables|Default|GetRight%20Shoes) false false))