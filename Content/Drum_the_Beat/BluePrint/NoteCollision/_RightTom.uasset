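; Right tom note collision Blueprint for the Drum the Beat game, scoring a point for notes that overlap the score bar.
; BeginPlay caches BarCollision from BP_JingleBellScore, tints AngelRing blue, calls BindScore and binds an event to BP_MasterDrum's right tom.
; AutoGenFunc scans Sphere0's overlapping components for that bar and increments the GameInstance's Point on a match.
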(event EventBeginPlay
  (Utilities|FlowControl|Sequence
    (:then_0
      (bind _returnvalue (Actor|GetActorOfClass "/Game/Drum_the_Beat/BluePrint/BP_JingleBellScore.BP_JingleBellScore_C"))
      (Variables|Default|SetBar%20Collision (Variables|/Game/Drum_the_Beat/BluePrint/BP_JingleBellScore.BP_JingleBellScore_C|GetBarCollision _returnvalue))
      (Rendering|Material|SetVectorParameterValueonMaterials (Variables|Default|GetAngelRing) "Rainbow" "0.000000,0.000000,1.000000")
      (CallFunction|BindScore))
    (:then_1
      (bind _returnvalue_2 (Actor|GetActorOfClass "/Game/Drum_the_Beat/BluePrint/Drum/BP_MasterDrum.BP_MasterDrum_C"))
      (EventDispatchers|BindEventtoRightTom _returnvalue_2 (EventDispatchers|CreateEvent :!event AutoGenFunc)))))

(fn ConstructionScript)

(fn AutoGenFunc
  (for _array_element (Class|PrimitiveComponent|GetOverlappingComponents (Variables|Default|GetSphere_0))
    (if (== _array_element (Variables|Default|GetBar%20Collision))
      (bind _asbp_game_instance (Utilities|Casting|CastToBP_GameInstance (Game|GetGameInstance)))
      (Math|Integer|IncrementInt (Variables|/Game/Drum_the_Beat/BluePrint/BP_GameInstance.BP_GameInstance_C|GetPoint _asbp_game_instance)))))