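; Note collision actor for the Drum the Beat game, with a toggleable beginner guide ring.
; BeginerGuide flips GuideOn and the AngelRing visibility; while the guide is on, Tick shows the ring only while ScoreCollision overlaps this actor.
; BindScore takes ScoreCollision from the BP_JingleBellScore actor, retrying on a short timer until that actor exists.
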(event EventTick
  (params (DeltaSeconds :type Float%20%28single-precision%29))
  (if (Variables|Default|GetGuideOn)
    (if (Collision|IsOverlappingActor (Variables|Default|GetScore%20Collision) self :!class /Script/Engine.PrimitiveComponent)
      (Rendering|SetVisibility (Variables|Default|GetAngelRing) true false)
      (else
        (Rendering|SetVisibility (Variables|Default|GetAngelRing) false false)))))

(event EventBeginerGuide
  (if (Variables|Default|GetGuideOn)
    (Rendering|SetVisibility (Variables|Default|GetAngelRing) false false)
    (Variables|Default|SetGuideOn false)
    (else
      (Rendering|SetVisibility (Variables|Default|GetAngelRing) true false)
      (Variables|Default|SetGuideOn true))))

(fn ConstructionScript)

(fn BindScore
  (bind _returnvalue (Actor|GetActorOfClass "/Game/Drum_the_Beat/BluePrint/BP_JingleBellScore.BP_JingleBellScore_C"))
  (Utilities|IsValid _returnvalue
    (:Is%20Valid
      (Variables|Default|SetScore%20Collision (Variables|/Game/Drum_the_Beat/BluePrint/BP_JingleBellScore.BP_JingleBellScore_C|GetScoreCollision _returnvalue)))
    (:Is%20Not%20Valid
      (Utilities|Time|SetTimerbyFunctionName 0 "BindScore" 0.1))))