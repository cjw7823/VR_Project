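; BP_MasterDrum is a playable drum kit actor with snare, toms and cymbals that sound when hit by a BP_DrumStick.
; On BeginPlay it spawns the kick pedal and hi-hat actors at marker components.
; Each piece's overlap event calls SoundByVelocity, which tests the stick's physics velocity against two thresholds.
; It plays nothing or one of two sounds, shared by all pieces, at the struck component's location.
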(event OnComponentBeginOverlap(SnareDrumShell)
  (params (OverlappedComponent :type Primitive%20Component%20Object%20Reference) (OtherActor :type Actor%20Object%20Reference) (OtherComp :type Primitive%20Component%20Object%20Reference) (OtherBodyIndex :type Integer) (bFromSweep :type Boolean) (SweepResult :type Hit%20Result%20Structure%20%28by%20ref%29))
  (bind _asstatic_mesh_component (Utilities|Casting|CastToStaticMeshComponent OverlappedComponent))
  (CallFunction|SoundbyVelocity _asstatic_mesh_component OtherActor))

(event OnComponentBeginOverlap(DrumShell)
  (params (OverlappedComponent :type Primitive%20Component%20Object%20Reference) (OtherActor :type Actor%20Object%20Reference) (OtherComp :type Primitive%20Component%20Object%20Reference) (OtherBodyIndex :type Integer) (bFromSweep :type Boolean) (SweepResult :type Hit%20Result%20Structure%20%28by%20ref%29))
  (bind _asstatic_mesh_component (Utilities|Casting|CastToStaticMeshComponent OverlappedComponent))
  (CallFunction|SoundbyVelocity _asstatic_mesh_component OtherActor))

(event OnComponentBeginOverlap(DrumShell1)
  (params (OverlappedComponent :type Primitive%20Component%20Object%20Reference) (OtherActor :type Actor%20Object%20Reference) (OtherComp :type Primitive%20Component%20Object%20Reference) (OtherBodyIndex :type Integer) (bFromSweep :type Boolean) (SweepResult :type Hit%20Result%20Structure%20%28by%20ref%29))
  (bind _asstatic_mesh_component (Utilities|Casting|CastToStaticMeshComponent OverlappedComponent))
  (CallFunction|SoundbyVelocity _asstatic_mesh_component OtherActor))

(event OnComponentBeginOverlap(FloorTom)
  (params (OverlappedComponent :type Primitive%20Component%20Object%20Reference) (OtherActor :type Actor%20Object%20Reference) (OtherComp :type Primitive%20Component%20Object%20Reference) (OtherBodyIndex :type Integer) (bFromSweep :type Boolean) (SweepResult :type Hit%20Result%20Structure%20%28by%20ref%29))
  (bind _asstatic_mesh_component (Utilities|Casting|CastToStaticMeshComponent OverlappedComponent))
  (CallFunction|SoundbyVelocity _asstatic_mesh_component OtherActor))

(event OnComponentBeginOverlap(Cymbal1)
  (params (OverlappedComponent :type Primitive%20Component%20Object%20Reference) (OtherActor :type Actor%20Object%20Reference) (OtherComp :type Primitive%20Component%20Object%20Reference) (OtherBodyIndex :type Integer) (bFromSweep :type Boolean) (SweepResult :type Hit%20Result%20Structure%20%28by%20ref%29))
  (bind _asstatic_mesh_component (Utilities|Casting|CastToStaticMeshComponent OverlappedComponent))
  (CallFunction|SoundbyVelocity _asstatic_mesh_component OtherActor))

(event OnComponentBeginOverlap(Cymbal3)
  (params (OverlappedComponent :type Primitive%20Component%20Object%20Reference) (OtherActor :type Actor%20Object%20Reference) (OtherComp :type Primitive%20Component%20Object%20Reference) (OtherBodyIndex :type Integer) (bFromSweep :type Boolean) (SweepResult :type Hit%20Result%20Structure%20%28by%20ref%29))
  (bind _asstatic_mesh_component (Utilities|Casting|CastToStaticMeshComponent OverlappedComponent))
  (CallFunction|SoundbyVelocity _asstatic_mesh_component OtherActor))

(event EventBeginPlay
  (bind _hi_hat_spawnspot (Variables|Default|GetHi-Hat_SpawnSpot))
  (Game|SpawnActorfromClass "/Game/Drum/BluePrint/BP_KickDrumPedal.BP_KickDrumPedal_C" (Math|Transform|MakeTransform (Transformation|GetWorldLocation (Variables|Default|GetPedal_SpawnSpot)) "0, 0, 0" "1,1,1") "Undefined" 0 0)
  (Game|SpawnActorfromClass "/Game/Drum/BluePrint/BP_Hi-Hat.BP_Hi-Hat_C" (Math|Transform|MakeTransform (Transformation|GetWorldLocation _hi_hat_spawnspot) (Transformation|GetWorldRotation _hi_hat_spawnspot) "1,1,1") "Undefined" 0 0))

(fn ConstructionScript)

(fn SoundbyVelocity
  (params (Static%20Mesh%20Component :type Static%20Mesh%20Component%20Object%20Reference) (Actor :type Actor%20Object%20Reference%20%28by%20ref%29))
  (bind _returnvalue (Transformation|GetWorldLocation Static%20Mesh%20Component))
  (bind _asbp_drum_stick (Utilities|Casting|CastToBP_DrumStick Actor))
  (bind _returnvalue_2 (Physics|GetPhysicsLinearVelocity (Variables|/Game/Drum/BluePrint/BP_DrumStick.BP_DrumStick_C|GetStaticMesh _asbp_drum_stick) "None"))
  (if (not (Math|Vector|VectorIsNearlyZero _returnvalue_2 (Variables|Default|GetIntensity_01)))
    (if (Math|Vector|VectorIsNearlyZero _returnvalue_2 (Variables|Default|GetIntensity_02))
      (Audio|SpawnSoundatLocation "/Engine/VREditor/Sounds/UI/Drop_Item_From_ContentBrowser.Drop_Item_From_ContentBrowser" _returnvalue "0, 0, 0" 1.0 1.0 0.0 0 0)
      (else
        (Audio|SpawnSoundatLocation "/Game/StarterContent/Audio/Collapse01.Collapse01" _returnvalue "0, 0, 0" 1.0 1.0 0.0 0 0)))))