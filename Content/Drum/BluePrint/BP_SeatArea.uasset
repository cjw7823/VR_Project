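; BP_SeatArea is a box trigger in the Drum content that signals whether the VR player is seated or standing.
; Begin and end overlaps of the VRPawn's CameraCollision with the box call SeatPlayer and StandPlayer, so head position sets the state.
; On BeginPlay it always calls SeatPlayer, as the branch condition is fixed to true and the initial overlap check is unused.
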(event OnComponentBeginOverlap(Box)
  (params (OverlappedComponent :type Primitive%20Component%20Object%20Reference) (OtherActor :type Actor%20Object%20Reference) (OtherComp :type Primitive%20Component%20Object%20Reference) (OtherBodyIndex :type Integer) (bFromSweep :type Boolean) (SweepResult :type Hit%20Result%20Structure%20%28by%20ref%29))
  (bind _asvrpawn (Utilities|Casting|CastToVRPawn (Game|Player|GetPlayerPawn 0)))
  (if (== OtherComp (Variables|/Game/VRTemplate/Blueprints/VRPawn.VRPawn_C|GetCameraCollision _asvrpawn))
    (Default|CallSeatPlayer)))

(event OnComponentEndOverlap(Box)
  (params (OverlappedComponent :type Primitive%20Component%20Object%20Reference) (OtherActor :type Actor%20Object%20Reference) (OtherComp :type Primitive%20Component%20Object%20Reference) (OtherBodyIndex :type Integer))
  (bind _asvrpawn (Utilities|Casting|CastToVRPawn (Game|Player|GetPlayerPawn 0)))
  (if (== OtherComp (Variables|/Game/VRTemplate/Blueprints/VRPawn.VRPawn_C|GetCameraCollision _asvrpawn))
    (Default|CallStandPlayer)))

(event EventBeginPlay
  (bind _asvrpawn (Utilities|Casting|CastToVRPawn (Game|Player|GetPlayerPawn 0)))
  (if true
    (Default|CallSeatPlayer)
    (else
      (Default|CallStandPlayer))))

(fn ConstructionScript)