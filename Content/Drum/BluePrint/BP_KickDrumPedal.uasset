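; Kick drum pedal Blueprint that animates a pedal press once when play begins.
; BeginPlay starts a fast looping timer that calls PushPedal by function name.
; Each tick steps pitch, X and Z toward fixed limits and applies them to Pedal2's relative transform.
; The timer clears itself once the pitch limit is reached, and the file contains no release motion.
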(event EventBeginPlay
  (Utilities|Time|SetTimerbyFunctionName 0 "PushPedal" 0.01 true))

(fn ConstructionScript)

(fn PushPedal
  (Utilities|FlowControl|Sequence
    (:then_0
      (if (> (Variables|Default|GetNew%20Rotation%20Y%20%28Pitch%29) -44.0)
        (Variables|Default|SetNew%20Rotation%20Y%20%28Pitch%29 (+ (Variables|Default|GetNew%20Rotation%20Y%20%28Pitch%29) -15.0))))
    (:then_1
      (if (> (Variables|Default|GetNew%20Location%20X) -15.0)
        (Variables|Default|SetNew%20Location%20X (+ (Variables|Default|GetNew%20Location%20X) -5.4))
        (Variables|Default|SetNew%20Location%20Z (+ (Variables|Default|GetNew%20Location%20Z) 1.5))))
    (:then_2
      (Transformation|SetRelativeLocationAndRotation (Variables|Default|GetPedal_2) (Math|Vector|MakeVector (Variables|Default|GetNew%20Location%20X) 0.0 (Variables|Default|GetNew%20Location%20Z)) (Math|Rotator|MakeRotator 0.0 (Variables|Default|GetNew%20Rotation%20Y%20%28Pitch%29) 0.0) false false)
      (if (<= (Variables|Default|GetNew%20Rotation%20Y%20%28Pitch%29) -44.0)
        (Utilities|Time|ClearTimerbyFunctionName 0 "PushPedal")))))